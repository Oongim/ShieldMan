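; BP_TitleUIPlayerController is the player controller for the title scene, showing the title UI and relaying login to the server.
; On BeginPlay it creates the UI_TitleScene widget, adds it to the viewport, shows the cursor and switches to UI-only input.
; ServerLogin passes the controller to BP_TitleGameMode's OnLogin.
; OnRepPlayerNumber copies the replicated PlayerNumber into SM_GameInstance.
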(event `self.ReceiveBeginPlay`
  (bind _returnvalue (`|CreateWidget` "/Game/UI/TitleScene/UI_TitleScene.UI_TitleScene_C" self))
  (bind _output_get (set `self.WGLogin` _returnvalue))
  (`UserWidget.AddToViewport` _output_get 0)
  (set `self.bShowMouseCursor` true)
  (`WidgetBlueprintLibrary.SetInputMode_UIOnlyEx` self _output_get))

(event `ServerLogin`
  (bind _asbp_title_game_mode (cast `/Game/0Title/BP_TitleGameMode` (`GameplayStatics.GetGameMode`)))
  (`/Game/0Title/BP_TitleGameMode.On Login` _asbp_title_game_mode self))

(fn `OnRepPlayerNumber`
  (bind _assm_game_instance (cast `SM_GameInstance` (`GameplayStatics.GetGameInstance`)))
  (`SM_GameInstance.SetPlayerNumber` _assm_game_instance (`self.PlayerNumber`)))

(fn `UserConstructionScript`)