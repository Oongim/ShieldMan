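; BP_CinematicDoor is a double door actor that swings open on its own, likely for a cinematic in Stage 1.
; Tick accumulates elapsed time in FDelta and, until it passes two seconds, adds opposite local yaw to the Left and Right components.
; Each frame's step equals the accumulated time, so the swing speeds up and depends on frame rate.
; BeginPlay, overlap and construction logic are empty.
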(event `self.ReceiveTick`
  (params (DeltaSeconds :type "Float (single-precision)"))
  (bind _returnvalue (* 1 (`self.fDelta`)))
  (bind _output_get (set `self.fDelta` (+ DeltaSeconds (`self.fDelta`))))
  (if (>= 2.0 _output_get)
    (`SceneComponent.K2_AddLocalRotation` (`self.Left`) (`KismetMathLibrary.MakeRotator` 0.0 0.0 _returnvalue) false false)
    (`SceneComponent.K2_AddLocalRotation` (`self.Right`) (`KismetMathLibrary.MakeRotator` 0.0 0.0 (* -1 _returnvalue)) false false)))

(fn `UserConstructionScript`)