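; Stage torch actor that switches its fire effect and point light on or off based on camera and character positions along the Y axis.
; While Isused is set, Tick hides both once when a CameraActor reaches 500 units past the torch in +Y, then clears Camerawork.
; Within that camera loop, it shows both again for any BP_SMCharacter no farther than 500 units past it in +Y.
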(event `self.ReceiveTick`
  (params (DeltaSeconds :type "Float (single-precision)"))
  (if (`self.isused`)
    (bind _outactors (`GameplayStatics.GetAllActorsOfClass` "/Script/Engine.CameraActor"))
    (for _array_element _outactors
      (if (and (`self.camerawork`) (>= (.y (`self.K2_GetActorLocation` _array_element)) (+ (.y (`self.K2_GetActorLocation`)) 500.0)))
        (`SceneComponent.SetVisibility` (`self.P_Torch_Fire`) false false)
        (`SceneComponent.SetVisibility` (`self.Torch_PointLight`) false false)
        (set `self.camerawork` false))
      (bind _outactors_2 (`GameplayStatics.GetAllActorsOfClass` "/Game/BP/BP_SMCharacter.BP_SMCharacter_C"))
      (for _array_element_2 _outactors_2
        (if (>= (.y (`self.K2_GetActorLocation`)) (+ (.y (`self.K2_GetActorLocation` _array_element_2)) -500.0))
          (`SceneComponent.SetVisibility` (`self.P_Torch_Fire`) true false)
          (`SceneComponent.SetVisibility` (`self.Torch_PointLight`) true false))))))

(fn `UserConstructionScript`)