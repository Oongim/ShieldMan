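; BP_SMCharacter1 is a character Blueprint that adds physical animation, hand collision and debug hotkeys.
; On BeginPlay it applies physical animation settings and simulates the bodies below a chosen bone, blending physics with animation.
; The construction script attaches left and right collision components to the Bip001 hand sockets.
; Keys lower HP, toggle an HP lock flag, teleport to fixed spots, or switch between the title and three stages.
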(event `self.ReceiveBeginPlay`
  (bind _physicalanimation (`self.PhysicalAnimation`))
  (bind _bone (`self.Bone`))
  (`PhysicalAnimationComponent.SetSkeletalMeshComponent` _physicalanimation (`self.Mesh`))
  (`PhysicalAnimationComponent.ApplyPhysicalAnimationSettingsBelow` _physicalanimation _bone (make `PhysicalAnimationData` false 10000.0 1000.0 100.0 100.0) false)
  (`SkeletalMeshComponent.SetAllBodiesBelowSimulatePhysics` (`self.Mesh`) _bone true false))

(event `Key|P`
  (params (Key :type "Key Structure"))
  (:`Pressed`
    (set `self.CurrentHP` (- (`self.CurrentHP`) 80.0))))

(event `Key|Seven`
  (params (Key :type "Key Structure"))
  (:`Pressed`
    (`self.SwitchLevel` "Stage1")))

(event `Key|Nine`
  (params (Key :type "Key Structure"))
  (:`Pressed`
    (`self.SwitchLevel` "Stage3")))

(event `Key|O`
  (params (Key :type "Key Structure"))
  (:`Pressed`
    (set `self.HPlock` true)))

(event `Key|Eight`
  (params (Key :type "Key Structure"))
  (:`Pressed`
    (`self.SwitchLevel` "Stage2")))

(event `Key|Zero`
  (params (Key :type "Key Structure"))
  (:`Pressed`
    (`self.SwitchLevel` "Title")))

(event `Key|I`
  (params (Key :type "Key Structure"))
  (:`Pressed`
    (set `self.HPlock` false)))

(event `Key|J`
  (params (Key :type "Key Structure"))
  (:`Pressed`
    (`self.K2_SetActorLocation` (-2000.0 300.0 100.0))))

(event `Key|K`
  (params (Key :type "Key Structure"))
  (:`Pressed`
    (`self.K2_SetActorLocation` (-4400.0 300.0 100.0))))

(fn `UserConstructionScript`
  (`SceneComponent.K2_AttachToComponent` (`self.Right_Collision`) (`self.Mesh`) "Bip001-R-Hand" "KeepRelative" "KeepRelative" "KeepRelative" true)
  (`SceneComponent.K2_AttachToComponent` (`self.Left_Collision`) (`self.Mesh`) "Bip001-L-Hand" "KeepRelative" "KeepRelative" "KeepRelative" true))