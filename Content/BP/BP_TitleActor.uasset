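; BP_TitleActor is a title actor whose Knight mesh moves a hand to follow the mouse cursor.
; Each Tick maps the DPI-scaled mouse position, relative to a hardcoded 1920x1080 center and divided by viewport size, to a HandPos vector.
; Vertical mouse movement drives X and horizontal drives Y, with Z fixed.
; The vector is written directly into the Knight's BP_SMTitleAnim animation instance.
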(event `self.ReceiveBeginPlay`)

(event `self.ReceiveTick`
  (params (DeltaSeconds :type "Float (single-precision)"))
  (bind (_locationx _locationy) (`WidgetLayoutLibrary.GetMousePositionScaledByDPI` (`GameplayStatics.GetPlayerController` 0)))
  (set `/Game/BP/Animation/BP_SMTitleAnim.Hand_Pos` (`KismetMathLibrary.MakeVector` (+ (* (/ (- _locationy 540.0) (`self.ViewportHeight`)) 35.0) -49.0) (* (/ (- _locationx 960.0) (`self.ViewportWidth`)) -60.0) 45.0) (cast `/Game/BP/Animation/BP_SMTitleAnim` (`SkeletalMeshComponent.GetAnimInstance` (`self.Knight`)) :!pure true)))

(fn `UserConstructionScript`)