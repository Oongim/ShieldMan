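; BP_SMGameMode is a multiplayer game mode that assigns player pawns and moves the session between stages.
; Pawn spawning gives a player BP_SMCharacter when none exists, otherwise BP_ArmPlayerPawn.
; Its servertravel event flags each character as ServerTraveling and copies the finished stage's value from SM_GameState into SM_GameInstance.
; It then runs a listen-server travel command to Stage2 or Stage3, all inside the per-character loop.
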(event `servertravel`
  (params (stage :type Name))
  (if (== stage "Stage2")
    (bind _outactors (`GameplayStatics.GetAllActorsOfClass` "/Game/BP/BP_SMCharacter.BP_SMCharacter_C"))
    (for _array_element _outactors
      (set `ShieldManCharacter.ServerTraveling` true _array_element)
      (bind _assm_game_instance (cast `SM_GameInstance` (`GameplayStatics.GetGameInstance`)))
      (bind _assm_game_state (cast `SM_GameState` (`GameplayStatics.GetGameState`)))
      (set `SM_GameInstance.Stage1` (`SM_GameState.Stage1` _assm_game_state) _assm_game_instance)
      (`KismetSystemLibrary.ExecuteConsoleCommand` "servertravel/Game/2Stage/Stage2?listen" null))
    (elif (== stage "Stage3")
      (bind _outactors_2 (`GameplayStatics.GetAllActorsOfClass` "/Game/BP/BP_SMCharacter.BP_SMCharacter_C"))
      (for _array_element_2 _outactors_2
        (set `ShieldManCharacter.ServerTraveling` true _array_element_2)
        (bind _assm_game_instance_2 (cast `SM_GameInstance` (`GameplayStatics.GetGameInstance`)))
        (bind _assm_game_state_2 (cast `SM_GameState` (`GameplayStatics.GetGameState`)))
        (set `SM_GameInstance.Stage2` (`SM_GameState.Stage2` _assm_game_state_2) _assm_game_instance_2)
        (`KismetSystemLibrary.ExecuteConsoleCommand` "servertravel/Game/3Stage/Stage3?listen" null)))))

(fn `SpawnDefaultPawnAtTransform`
  (params (NewPlayer :type "Controller Object Reference") (SpawnTransform :type "Transform Structure (by ref)"))
  (returns (ReturnValue :type "Pawn Object Reference"))
  (bind _outactors (`GameplayStatics.GetAllActorsOfClass` "/Game/BP/BP_SMCharacter.BP_SMCharacter_C"))
  (if (== (`KismetArrayLibrary.Array_Length` _outactors) 0)
    (bind _returnvalue (`|SpawnActorFromClass` "/Game/BP/BP_SMCharacter.BP_SMCharacter_C" SpawnTransform "Undefined" "OverrideRootScale" null null))
    (return _returnvalue)
    (else
      (bind _returnvalue_2 (`|SpawnActorFromClass` "/Game/BP/BP_ArmPlayerPawn.BP_ArmPlayerPawn_C" SpawnTransform "Undefined" "OverrideRootScale" null null))
      (return _returnvalue_2))))

(fn `UserConstructionScript`)