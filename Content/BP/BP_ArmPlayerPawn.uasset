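; BP_ArmPlayerPawn is a player pawn Blueprint that handles gameplay UI and network leave notification.
; BeginPlay adds the UI_PlayScene widget to the viewport, and CallLoading adds UI_Loading.
; On Destroyed, it checks every BP_SMCharacter and sends a leave packet through the SM_GameInstance network manager for each with depleted HP.
; For living characters, it instead sends one per cleared BP_MetaBall_Boss while connected.
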(event `self.ReceiveBeginPlay`
  (bind _returnvalue (`|CreateWidget` "/Game/UI/PlayScene/UI_PlayScene.UI_PlayScene_C"))
  (`UserWidget.AddToViewport` _returnvalue 0))

(event `self.Call_Loading`
  (bind _returnvalue (`|CreateWidget` "/Game/UI/PlayScene/UI_Loading.UI_Loading_C"))
  (`UserWidget.AddToViewport` _returnvalue 0))

(event `self.ReceiveDestroyed`
  (bind _outactors (`GameplayStatics.GetAllActorsOfClass` "/Game/BP/BP_SMCharacter.BP_SMCharacter_C"))
  (for _array_element _outactors
    (if (<= (`ShieldManCharacter.CurrentHP` _array_element) 0.0)
      (bind _assm_game_instance (cast `SM_GameInstance` (`GameplayStatics.GetGameInstance`)))
      (bind _returnvalue (`SM_GameInstance.GetNetworkManager` _assm_game_instance))
      (`NetworkManager.Send_Leave_Packet` _returnvalue)
      (else
        (bind _outactors_2 (`GameplayStatics.GetAllActorsOfClass` "/Game/BP/3Stage/BP_MetaBall_Boss.BP_MetaBall_Boss_C"))
        (for _array_element_2 _outactors_2
          (if (`/Game/BP/3Stage/BP_MetaBall_Boss.isclear` _array_element_2)
            (bind _assm_game_instance_2 (cast `SM_GameInstance` (`GameplayStatics.GetGameInstance`)))
            (bind _returnvalue_2 (`SM_GameInstance.GetNetworkManager` _assm_game_instance_2))
            (if (`NetworkManager.isConnect` _returnvalue_2)
              (`NetworkManager.Send_Leave_Packet` _returnvalue_2))))))))

(fn `UserConstructionScript`)