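; BP_SMCharacter is a character with physically animated bodies and collision components on both hands.
; On BeginPlay it applies world-space physical animation with strong drives and simulates physics on bodies below a configured bone, excluding the bone itself.
; The construction script attaches the left and right collision components to the mesh's hand sockets.
; Pressing P subtracts a fixed amount from CurrentHP.
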(event `self.ReceiveBeginPlay`
  (bind _physicalanimation (`self.PhysicalAnimation`))
  (bind _bone (`self.Bone`))
  (`PhysicalAnimationComponent.SetSkeletalMeshComponent` _physicalanimation (`self.Mesh`))
  (`PhysicalAnimationComponent.ApplyPhysicalAnimationSettingsBelow` _physicalanimation _bone (make `PhysicalAnimationData` false 10000.0 1000.0 10000.0 100.0) false)
  (`SkeletalMeshComponent.SetAllBodiesBelowSimulatePhysics` (`self.Mesh`) _bone true false))

(event `Key|P`
  (params (Key :type "Key Structure"))
  (:`Pressed`
    (set `self.CurrentHP` (- (`self.CurrentHP`) 80.0))))

(fn `UserConstructionScript`
  (`SceneComponent.K2_AttachToComponent` (`self.Right_Collision`) (`self.Mesh`) "Bip001-R-Hand" "KeepRelative" "KeepRelative" "KeepRelative" true)
  (`SceneComponent.K2_AttachToComponent` (`self.Left_Collision`) (`self.Mesh`) "Bip001-L-Hand" "KeepRelative" "KeepRelative" "KeepRelative" true))